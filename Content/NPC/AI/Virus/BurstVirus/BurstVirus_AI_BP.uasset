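; AI controller for the BurstVirus NPC that sets up its blackboard on BeginPlay and starts its behavior tree once the possessed virus reports ready.
; Every tick it polls that readiness and mirrors the pawn's CellToInfect into the blackboard, with debug prints.
; The key is set only while empty and cleared only when the pawn's cell becomes invalid, so switching between valid cells does not update it.
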(event EventBeginPlay
  (bind _blackboardcomponent (Class|AIController|UseBlackboard "/Game/NPC/AI/Virus/BurstVirus/BurstVirus_Blackboard.BurstVirus_Blackboard"))
  (Variables|Default|SetBlackboardComp _blackboardcomponent))

(event EventTick
  (params (DeltaSeconds :type Float%20%28single-precision%29))
  (CallFunction|CheckifVirusReady)
  (Utilities|IsValid (AI|Components|Blackboard|GetValueasObject (Variables|Default|GetBlackboardComp) (Variables|Default|GetInfectableVirusKey))
    (:Is%20Valid
      (CallFunction|ClearInfectableCellinBlackboard))
    (:Is%20Not%20Valid
      (CallFunction|SetInfectableCellinBlackboard))))

(fn ConstructionScript)

(fn CheckifVirusReady
  (bind _asvirus (Utilities|Casting|CastToVirus (Pawn|GetControlledPawn)))
  (if (and (Variables|/Script/VirusForce.Virus|GetIsVirusReady _asvirus) (not (Variables|Default|GetIsBehaviorRunning)))
    (AI|RunBehaviorTree "/Game/NPC/AI/Virus/BurstVirus/BurstVirus_Behavior.BurstVirus_Behavior")
    (Variables|Default|SetIsBehaviorRunning true)))

(fn SetInfectableCellinBlackboard
  (bind _asburst_virus (Utilities|Casting|CastToBurstVirus (Pawn|GetControlledPawn)))
  (Utilities|IsValid (Variables|/Script/VirusForce.BurstVirus|GetCellToInfect _asburst_virus)
    (:Is%20Valid
      (AI|Components|Blackboard|SetValueasObject (Variables|Default|GetBlackboardComp) (Variables|Default|GetInfectableVirusKey) (Variables|/Script/VirusForce.BurstVirus|GetCellToInfect _asburst_virus))
      (Development|PrintString "Set infectable cell"))))

(fn ClearInfectableCellinBlackboard
  (bind _asburst_virus (Utilities|Casting|CastToBurstVirus (Pawn|GetControlledPawn)))
  (Utilities|IsValid (Variables|/Script/VirusForce.BurstVirus|GetCellToInfect _asburst_virus)
    (:Is%20Not%20Valid
      (Development|PrintString "Attempting to clear")
      (AI|Components|Blackboard|ClearValue (Variables|Default|GetBlackboardComp) (Variables|Default|GetInfectableVirusKey))
      (Development|PrintString "Cleared targets"))))