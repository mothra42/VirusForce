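; AI controller for the Virus NPC that holds off its behavior until the controlled virus reports it is ready.
; BeginPlay sets up Virus_Blackboard.
; Tick polls IsVirusReady on the possessed Virus pawn and starts Virus_Behavior once, guarded by the IsBehaviorRunning flag.
; A second, unconnected RunBehaviorTree node never runs.
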(event EventBeginPlay
  (Class|AIController|UseBlackboard "/Game/NPC/AI/Virus/BaseVirus/Virus_Blackboard.Virus_Blackboard"))

(event EventTick
  (params (DeltaSeconds :type Float%20%28single-precision%29))
  (bind _asvirus (Utilities|Casting|CastToVirus (Pawn|GetControlledPawn)))
  (if (and (Variables|/Script/VirusForce.Virus|GetIsVirusReady _asvirus) (not (Variables|Default|GetIsBehaviorRunning)))
    (AI|RunBehaviorTree "/Game/NPC/AI/Virus/BaseVirus/Virus_Behavior.Virus_Behavior")
    (Variables|Default|SetIsBehaviorRunning true)))

(fn ConstructionScript)