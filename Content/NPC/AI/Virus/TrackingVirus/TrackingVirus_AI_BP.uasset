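; AI controller for the tracking virus NPC that starts its behavior tree once the virus is ready.
; On BeginPlay it sets up the TrackingVirus blackboard and stores the player pawn under the player key.
; Each tick it checks the controlled Virus pawn's ready flag and runs the tracking behavior tree a single time, guarded by a running flag.
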(event EventBeginPlay
  (bind _blackboardcomponent (Class|AIController|UseBlackboard "/Game/NPC/AI/Virus/TrackingVirus/TrackingVirusBlackboard.TrackingVirusBlackboard"))
  (bind _output_get (Variables|Default|SetBlackboardComp _blackboardcomponent))
  (AI|Components|Blackboard|SetValueasObject _output_get (Variables|Default|GetPlayerKey) (Game|Player|GetPlayerPawn 0)))

(event EventTick
  (params (DeltaSeconds :type Float%20%28single-precision%29))
  (CallFunction|CheckifVirusReady))

(fn ConstructionScript)

(fn CheckifVirusReady
  (bind _asvirus (Utilities|Casting|CastToVirus (Pawn|GetControlledPawn)))
  (if (and (Variables|/Script/VirusForce.Virus|GetIsVirusReady _asvirus) (not (Variables|Default|GetIsBehaviorRunning)))
    (AI|RunBehaviorTree "/Game/NPC/AI/Virus/TrackingVirus/TackingVirusBehaviorTree.TackingVirusBehaviorTree")
    (Variables|Default|SetIsBehaviorRunning true)))